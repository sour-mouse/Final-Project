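; BP_Player is the player for a rhythm game, holding Life and Score and taking four color-coded inputs.
; On BeginPlay it adds the rhythm Enhanced Input mapping context; each color action finds BP_Spline in the level and passes it a button index.
; DamagePlayer and HealPlayer adjust clamped Life, with depletion opening the GameOver level.
; IncrementScore adds a given amount to Score.
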(event Input|EnhancedActionEvents|EnhancedInputActionIA_Cyan
  (params (ActionValue :type Boolean) (ElapsedSeconds :type Float%20%28double-precision%29) (TriggeredSeconds :type Float%20%28double-precision%29) (InputAction :type Input%20Action%20Object%20Reference :default "/Game/Inputs/Actions/IA_Cyan.IA_Cyan"))
  (:Started
    (bind _returnvalue (Actor|GetActorOfClass "/Game/GameAssets/BP_Spline.BP_Spline_C"))
    (Default|ButtonPressed _returnvalue)))

(event Input|EnhancedActionEvents|EnhancedInputActionIA_Pink
  (params (ActionValue :type Boolean) (ElapsedSeconds :type Float%20%28double-precision%29) (TriggeredSeconds :type Float%20%28double-precision%29) (InputAction :type Input%20Action%20Object%20Reference :default "/Game/Inputs/Actions/IA_Pink.IA_Pink"))
  (:Started
    (bind _returnvalue (Actor|GetActorOfClass "/Game/GameAssets/BP_Spline.BP_Spline_C"))
    (Default|ButtonPressed _returnvalue 1)))

(event Input|EnhancedActionEvents|EnhancedInputActionIA_Yellow
  (params (ActionValue :type Boolean) (ElapsedSeconds :type Float%20%28double-precision%29) (TriggeredSeconds :type Float%20%28double-precision%29) (InputAction :type Input%20Action%20Object%20Reference :default "/Game/Inputs/Actions/IA_Yellow.IA_Yellow"))
  (:Started
    (bind _returnvalue (Actor|GetActorOfClass "/Game/GameAssets/BP_Spline.BP_Spline_C"))
    (Default|ButtonPressed _returnvalue 2)))

(event Input|EnhancedActionEvents|EnhancedInputActionIA_Green
  (params (ActionValue :type Boolean) (ElapsedSeconds :type Float%20%28double-precision%29) (TriggeredSeconds :type Float%20%28double-precision%29) (InputAction :type Input%20Action%20Object%20Reference :default "/Game/Inputs/Actions/IA_Green.IA_Green"))
  (:Started
    (bind _returnvalue (Actor|GetActorOfClass "/Game/GameAssets/BP_Spline.BP_Spline_C"))
    (Default|ButtonPressed _returnvalue 3)))

(event EventBeginPlay
  ;[0.15 0.15 0.15 0.5] Inputs
  (bind _asplayer_controller (Utilities|Casting|CastToPlayerController (Pawn|GetController)))
  (Utilities|IsValid (PlayerController|LocalPlayerSubsystems|GetEnhancedInputLocalPlayerSubsystem _asplayer_controller)
    (:Is%20Valid
      (Input|AddMappingContext (PlayerController|LocalPlayerSubsystems|GetEnhancedInputLocalPlayerSubsystem _asplayer_controller) "/Game/Inputs/IMC_RhythmMapping.IMC_RhythmMapping" 0 "(bIgnoreAllPressedKeysUntilRelease=True,bForceImmediately=False,bNotifyUserSettings=False)"))))

(fn ConstructionScript)

(fn DamagePlayer
  (if (> (Variables|Default|GetLife) 0)
    (Variables|Default|SetLife (Math|Integer|Clamp(Integer) (- (Variables|Default|GetLife) 10) 0 100))
    (if (not (> (Variables|Default|GetLife) 0))
      (Game|OpenLevel(byObjectReference) "/Game/Maps/GameOver.GameOver"))))

(fn HealPlayer
  (if (> (Variables|Default|GetLife) 0)
    (Variables|Default|SetLife (Math|Integer|Clamp(Integer) (+ (Variables|Default|GetLife) 2) 0 100))))

(fn IncrementScore
  (params (Amount :type Integer))
  (if true
    (Variables|Default|SetScore (+ (Variables|Default|GetScore) Amount))))