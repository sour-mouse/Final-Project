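; BP_Note1 is a note actor that travels along a spline lane and can report misses.
; MoveNotes runs a timeline at a play rate of 1/CompletionTime, lerping distance along the given lane to set world position and rotation while keeping the sphere's relative scale.
; UpdateMisses forwards its value to BP_PlayerState.
; BeginPlay caches the level's BP_Spline actor, though this graph does not use it afterward.
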(event Custom|MoveNotes
  (params (Lane :type Spline%20Component%20Object%20Reference))
  (Components|Timeline|SetPlayRate (Variables|Default|GetTimeline) (/ 1.0 (Variables|Default|GetCompletionTime)))
  (bind _newtrack_0 (Timeline|Timeline PlayFromStart)
    (:Update
      (Transformation|SetActorTransform (Math|Transform|MakeTransform (Spline|GetLocationatDistanceAlongSpline Lane (Math|Float|Lerp 0.0 (Spline|GetSplineLength Lane) _newtrack_0) "World") (Spline|GetRotationatDistanceAlongSpline Lane (Math|Float|Lerp 0.0 (Spline|GetSplineLength Lane) _newtrack_0) "World") (Variables|/Script/Engine.SceneComponent|GetRelativeScale3D (Variables|Default|GetSphere)))))))

(event EventBeginPlay
  (bind _returnvalue (Actor|GetActorOfClass "/Game/GameAssets/BP_Spline.BP_Spline_C"))
  (Variables|Default|SetGameSpline _returnvalue))

(event EventUpdateMisses
  (params (Value :type Integer))
  (Default|UpdateMisses (.AsBP%20Player%20State (Utilities|Casting|CastToBP_PlayerState (Game|GetPlayerState 0))) Value))

(fn ConstructionScript)