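; Player state for a rhythm game that tracks the player's score and a miss counter that doubles as lives.
; UpdateScore adds to the running score, copies it to BP_RhythmGameInstance and refreshes the in-game UI through BP_PlayerController.
; UpdateMisses adds to the miss counter and refreshes the same widget.
; ResetPlayerData zeroes the score and sets the miss counter to DefaultLives.
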(event EventBeginPlay)

(event EventTick
  (params (DeltaSeconds :type Float%20%28single-precision%29)))

(event EventUpdateScore
  (params (Value :type Integer))
  (bind _self self)
  (bind _returnvalue (Game|GetPlayerController _self))
  (bind (_asbp_player_controller _bsuccess) (Utilities|Casting|CastToBP_PlayerController _returnvalue))
  ;[0.15 0.15 0.15 0.5] Update Score
  (bind _output_get (Variables|CurrentGame|SetCurrentScore (+ Value (Variables|CurrentGame|GetCurrentScore))))
  (bind _asbp_rhythm_game_instance (Utilities|Casting|CastToBP_RhythmGameInstance (Game|GetGameInstance)))
  (Variables|/Game/GameAssets/BP_RhythmGameInstance.BP_RhythmGameInstance_C|SetGameScore _asbp_rhythm_game_instance _output_get)
  (if _bsuccess
    (Default|SetCurrentScore (Variables|/Game/Blueprints/BP_PlayerController.BP_PlayerController_C|GetWidgetInGameUI _asbp_player_controller))))

(event EventUpdateMisses
  (params (Value :type Integer))
  (bind _self self)
  (bind _returnvalue (Game|GetPlayerController _self))
  (bind (_asbp_player_controller _bsuccess) (Utilities|Casting|CastToBP_PlayerController _returnvalue))
  ;[0.15 0.15 0.15 0.5] Update Lives
  (Variables|CurrentGame|SetCurrentMisses (+ Value (Variables|CurrentGame|GetCurrentMisses)))
  (if _bsuccess
    (Default|SetCurrentMisses (Variables|/Game/Blueprints/BP_PlayerController.BP_PlayerController_C|GetWidgetInGameUI _asbp_player_controller))))

(fn ConstructionScript)

(fn ResetPlayerData
  (Variables|CurrentGame|SetCurrentScore 0)
  (Variables|CurrentGame|SetCurrentMisses (Variables|DefaultSettings|GetDefaultLives)))