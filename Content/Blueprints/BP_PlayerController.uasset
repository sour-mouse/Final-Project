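; Player controller that manages input setup, the in-game HUD and the pause menu.
; SetupController checks the pawn for BPI_PlayerInterface, adds the Enhanced Input mapping, shows the HUD and saves the pawn transform as CurrentSpawn in BP_PlayerState.
; The pause action swaps the HUD for a menu, pauses and switches to UI-only input; ResumeGame reverses this, reusing the cached HUD widget.
; Cleanup removes the mapping and clears the interface reference.
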(event Input|EnhancedActionEvents|EnhancedInputActionIA_PauseGame
  (params (ActionValue :type Boolean) (ElapsedSeconds :type Float%20%28double-precision%29) (TriggeredSeconds :type Float%20%28double-precision%29) (InputAction :type Input%20Action%20Object%20Reference :default "/Game/Inputs/Actions/IA_PauseGame.IA_PauseGame"))
  ;[0.15 0.15 0.15 0.5] Pause Game
  (Widget|RemovefromParent (Variables|InGameUI|GetWidgetInGameUI))
  (bind _returnvalue (UserInterface|CreateWidget "/Game/UI/UMG_InGamePauseMenu.UMG_InGamePauseMenu_C" self))
  (bind _output_get (Variables|Default|SetWidgetInGameMenu _returnvalue))
  (UserInterface|Viewport|AddtoViewport _output_get 0)
  (Input|SetInputModeUIOnly self (Variables|Default|GetWidgetInGameMenu) "DoNotLock" false)
  (Game|SetGamePaused true)
  (Variables|Default|SetbShowMouseCursor self true))

(event EventBeginPlay)

(event EventTick
  (params (DeltaSeconds :type Float%20%28single-precision%29)))

(event EventResumeGame
  ;[0.15 0.15 0.15 0.5] Pause Game
  (Utilities|IsValid (Variables|Default|GetWidgetInGameMenu)
    (:Is%20Valid
      (Widget|RemovefromParent (Variables|Default|GetWidgetInGameMenu))
      (Input|SetInputModeGameOnly self false)
      (Game|SetGamePaused false)
      (CallFunction|SetupinGameUI)
      (Variables|Default|SetbShowMouseCursor self false))))

(fn ConstructionScript)

(fn SetupController
  (bind _returnvalue (Pawn|GetControlledPawn))
  (bind _self self)
  (bind _returnvalue_2 (PlayerController|LocalPlayerSubsystems|GetEnhancedInputLocalPlayerSubsystem _self))
  (Game|SetGamePaused false)
  (bind _asbpi_player_interface (Utilities|Casting|CastToBPI_PlayerInterface _returnvalue)
    (:then
      (Variables|Default|SetPlayerInterface _asbpi_player_interface)
      (Utilities|IsValid _returnvalue_2
        (:Is%20Valid
          (Input|AddMappingContext _returnvalue_2 0 0 "(bIgnoreAllPressedKeysUntilRelease=True,bForceImmediately=False,bNotifyUserSettings=False)")
          (Input|SetInputModeGameOnly self false)
          (CallFunction|SetupinGameUI)
          (bind _asbp_player_state (Utilities|Casting|CastToBP_PlayerState (Variables|GetPlayerState self)))
          (Variables|/Game/Blueprints/BP_PlayerState.BP_PlayerState_C|SetCurrentSpawn _asbp_player_state (Transformation|GetActorTransform (Pawn|GetControlledPawn))))))
    (:CastFailed
      (Development|PrintString (Utilities|String|Append (Utilities|String|ToString(Object) _returnvalue) "Does Not Have Player Interface") true true "(R=1.000000,G=0.000000,B=0.000000,A=1.000000)"))))

(fn SetupinGameUI
  (if (Variables|InGameUI|GetHasGameUIBeenSetup)
    (Utilities|IsValid (Variables|InGameUI|GetWidgetInGameUI)
      (:Is%20Valid
        (if (not (Widget|IsVisible (Variables|InGameUI|GetWidgetInGameUI)))
          (UserInterface|Viewport|AddtoViewport (Variables|InGameUI|GetWidgetInGameUI) 0))))
    (else
      (bind _returnvalue (UserInterface|CreateWidget "/Game/UI/UMG_InGameUI.UMG_InGameUI_C" self))
      (bind _output_get (Variables|InGameUI|SetWidgetInGameUI _returnvalue))
      (UserInterface|Viewport|AddtoViewport _output_get 0)
      (Variables|InGameUI|SetHasGameUIBeenSetup true))))

(fn Cleanup
  (bind _self self)
  (bind _returnvalue (PlayerController|LocalPlayerSubsystems|GetEnhancedInputLocalPlayerSubsystem _self))
  (Utilities|IsValid _returnvalue
    (:Is%20Valid
      (Input|RemoveMappingContext _returnvalue 0 "(bIgnoreAllPressedKeysUntilRelease=True,bForceImmediately=False,bNotifyUserSettings=False)")
      (Variables|Default|SetPlayerInterface 0))))